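; Footstep anim notify that plays a surface-dependent sound when an animation hits the notify.
; Traces downward on Visibility around the left or right ball socket, chosen by the Right flag, ignoring the mesh's owner.
; On a hit, the physical material's surface type picks the walking, wood or gravel cue, played at the impact point with strong attenuation.
; SFXIndex selects the volume, including a silent option.
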(fn `Received_Notify`
  (params (MeshComp :type "SkeletalMeshComponent Object Reference") (Animation :type "AnimSequenceBase Object Reference") (EventReference :type "AnimNotifyEventReference Structure (by ref)"))
  (returns (ReturnValue :type Boolean))
  (bind _returnvalue (`SceneComponent.GetSocketLocation` MeshComp (select `bool` (`self.Right?`) :`false` "ball_l" :`true` "ball_r" :!type "Name")))
  (bind (_outhit _returnvalue_2) (`KismetSystemLibrary.LineTraceSingle` (+ _returnvalue (0.0 0.0 10.0)) (- _returnvalue (0.0 0.0 50.0)) "TraceTypeQuery1" false (`|MakeArray` (`ActorComponent.GetOwner` MeshComp))))
  (if _returnvalue_2
    (bind (_bblockinghit _binitialoverlap _time _distance _location _impactpoint _normal _impactnormal _physmat) (`GameplayStatics.BreakHitResult` _outhit))
    (`GameplayStatics.PlaySoundAtLocation` (select `EPhysicalSurface` (`PhysicalMaterial.SurfaceType` _physmat) :`SurfaceType_Default` "/Game/Sounds/FoleyEffects/Carpet/Cue_Walking.Cue_Walking" :`SurfaceType1` "/Game/Sounds/FoleyEffects/Carpet/Cue_Walking.Cue_Walking" :`SurfaceType2` "/Game/Sounds/FoleyEffects/Wood/Cue_Wood.Cue_Wood" :`SurfaceType3` "/Game/Sounds/FoleyEffects/Gravel/Cue_Gravel.Cue_Gravel" :!type "SoundBase Object Reference") _location (struct) (select `int` (`self.SFX Index`) :`0` 0.0 :`1` 0.25 :`2` 0.6 :!type "Float (single-precision)") 1.0 0.0 "/Game/Sounds/SA_Strong.SA_Strong" null null null)))