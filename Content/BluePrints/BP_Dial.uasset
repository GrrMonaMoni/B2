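; BP_Dial is one rotating digit dial of a lock, with ten positions 36 degrees apart.
; RotateDial plays a switch sound and a timeline that yaws the mesh one step, ignoring repeat calls until it finishes.
; On finish it wraps at 360, derives Number from the rotation and has LockRef check the lock.
; On BeginPlay it passes itself to its WBP_LockArrow widget.
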(event `FindNumber`
  (set `self.Number` (`KismetMathLibrary.FTrunc` (/ (`self.DialRotation`) 36.0))))

(event `RotateDial`
  (if (`self.CanRotate`)
    (set `self.CanRotate` false)
    (`GameplayStatics.PlaySound2D` "/Engine/VREditor/Sounds/UI/Flashlight_Switch.Flashlight_Switch" 1.0 1.0 0.0 null null)
    (bind (_direction _alpha) (`Timeline|DialRotation_TL` :!via `PlayFromStart`)
      (:`Update`
        (bind _returnvalue (+ (`self.DialRotation`) (`KismetMathLibrary.Lerp` 0.0 36.0 _alpha)))
        (`SceneComponent.K2_SetRelativeRotation` (`self.SM_DIalV3`) (`KismetMathLibrary.MakeRotator` 0.0 0.0 _returnvalue) false false))
      (:`Finished`
        (set `self.DialRotation` _returnvalue)
        (if (>= (`self.DialRotation`) 360.0)
          (set `self.DialRotation` 0.0)
          (`SceneComponent.K2_SetRelativeRotation` :`self` (`self.SM_DIalV3`)))
        (`self.FindNumber`)
        (`/Game/BluePrints/InteractBP_Children/BP_CombinationLock.Checkeveryturn` (`self.LockRef`))
        (set `self.CanRotate` true)))))

(event `self.ReceiveBeginPlay`
  (bind _aswbp_lock_arrow (cast `/Game/BluePrints/Widget_BP/Lock/WBP_LockArrow` (`WidgetComponent.GetUserWidgetObject` (`self.Arrow`))))
  (`/Game/BluePrints/Widget_BP/Lock/WBP_LockArrow.Initialse` _aswbp_lock_arrow self))

(fn `UserConstructionScript`)