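; BP_BaseNote is an interactable note that the player can pick up to read and put back down.
; Overlapping its Box toggles an outline overlay material on the Re component.
; Interact uses a FlipFlop to alternate between showing a WBP_TutNote widget and calling PutNoteDown on it.
; Each side plays a paper sound, toggles look and move input, and hides or restores Re and Widget.
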(event `self.Box.OnComponentBeginOverlap`
  (params (OverlappedComponent :type "PrimitiveComponent Object Reference") (OtherActor :type "Actor Object Reference") (OtherComp :type "PrimitiveComponent Object Reference") (OtherBodyIndex :type Integer) (bFromSweep :type Boolean) (SweepResult :type "HitResult Structure (by ref)"))
  ;[0.07738 0.08741 0.15 0.5] Show E Widget
  (`MeshComponent.SetOverlayMaterial` (`self.re`) "/Game/Materials/M_Outline.M_Outline"))

(event `self.Box.OnComponentEndOverlap`
  (params (OverlappedComponent :type "PrimitiveComponent Object Reference") (OtherActor :type "Actor Object Reference") (OtherComp :type "PrimitiveComponent Object Reference") (OtherBodyIndex :type Integer))
  ;[0.07738 0.08741 0.15 0.5] Show E Widget
  (`MeshComponent.SetOverlayMaterial` (`self.re`) null))

(event `/Game/BluePrints/BPI_PlayerInteract.Interact`
  (bind _returnvalue (`GameplayStatics.GetPlayerController` 0))
  (bind _re (`self.re`))
  (bind _returnvalue_2 (`SceneComponent.K2_GetComponentLocation` (`self.re`)))
  ;[0.15 0.1068 0.0633 0.5] Add and Remove Note
  (`/Engine/EditorBlueprintResources/StandardMacros.FlipFlop`
    (:`A`
      (`GameplayStatics.PlaySoundAtLocation` "/Game/Sounds/Paper/Paper1.Paper1" _returnvalue_2 (struct) 1.0 1.0 0.0 null null null null)
      (bind _returnvalue_3 (`|CreateWidget` "/Game/BluePrints/Widget_BP/Items/Notes/WBP_TutNote.WBP_TutNote_C"))
      (`UserWidget.AddToViewport` _returnvalue_3 0)
      (`Controller.SetIgnoreLookInput` _returnvalue true)
      (`Controller.SetIgnoreMoveInput` _returnvalue true)
      (`SceneComponent.SetVisibility` _re false false)
      (`SceneComponent.SetVisibility` (`self.Widget`) false false))
    (:`B`
      (`GameplayStatics.PlaySoundAtLocation` "/Game/Sounds/Paper/paper2.paper2" _returnvalue_2 (struct) 1.0 1.0 0.0 null null null null)
      (`/Game/BluePrints/Widget_BP/Items/Notes/WBP_TutNote.PutNoteDown` _returnvalue_3)
      (`Controller.SetIgnoreLookInput` _returnvalue false)
      (`Controller.SetIgnoreMoveInput` _returnvalue false)
      (`SceneComponent.SetVisibility` _re true false)
      (`SceneComponent.SetVisibility` (`self.Widget`) true false))))

(fn `UserConstructionScript`
  (`parent.UserConstructionScript`))