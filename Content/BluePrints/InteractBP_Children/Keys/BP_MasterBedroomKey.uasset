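; BP_MasterBedroomKey is a key pickup, apparently for the master bedroom, that the player collects by interacting with it.
; BeginPlay caches the player's BP_FirstPersonCharacter.
; On Interact it adds its KeyID to that character's keys, plays a pickup sound at its location, adds a widget to the viewport, then destroys itself.
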(event `self.ReceiveBeginPlay`
  (bind _asbp_first_person_character (cast `/Game/FirstPerson/Blueprints/BP_FirstPersonCharacter` (`GameplayStatics.GetPlayerCharacter` 0)))
  (set `self.Player Ref` _asbp_first_person_character))

(event `self.Interact`
  ;[0.15 0.07611 0.1383 0.5] Pick up key
  (`/Game/FirstPerson/Blueprints/BP_FirstPersonCharacter.AddKeys` (`self.Player Ref`) (`self.KeyID`))
  (`GameplayStatics.PlaySoundAtLocation` "/Game/Sounds/Door/Pickingupkey.Pickingupkey" (`SceneComponent.K2_GetComponentLocation` (`self.re`)) (struct) 1.0 1.0 0.0 null null null null)
  (bind _returnvalue (`|CreateWidget` (`self.Class`)))
  (`UserWidget.AddToViewport` _returnvalue 0)
  (`self.K2_DestroyActor`))

(fn `UserConstructionScript`
  (`parent.UserConstructionScript`))