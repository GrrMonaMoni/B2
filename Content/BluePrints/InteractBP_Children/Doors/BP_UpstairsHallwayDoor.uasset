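; Interactable upstairs hallway door that can be locked behind a key ID and swings open away from the player.
; Interact shows a door widget, then either toggles the door or compares the player's Keys against DoorKeyID to unlock it or show a locked prompt.
; A timeline drives the yaw, with direction picked by a dot product against the door's right vector.
; A looping timer closes it once the player moves beyond CloseDistance.
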(event `self.ReceiveBeginPlay`
  (bind _asbp_first_person_character (cast `/Game/FirstPerson/Blueprints/BP_FirstPersonCharacter` (`GameplayStatics.GetPlayerCharacter` 0)))
  (set `self.Player Ref` _asbp_first_person_character)
  (`self.AutoClose`))

(event `self.Interact`
  ; Interaction
  (bind _returnvalue (`|CreateWidget` "/Game/BluePrints/Widget_BP/Doors/WBP_LivingroomDoor.WBP_LivingroomDoor_C"))
  (set `self.DoorRef` _returnvalue)
  (`UserWidget.AddToViewport` _returnvalue 0)
  (if (`self.Locked?`)
    (`self.CheckForKey`)
    (else
      (`self.OpenCloseDoor`)
      (`Widget.RemoveFromParent` (`self.DoorRef`)))))

(event `DoorIsLocked`
  ;[0.15 0.04002 0.07429 0.5] It's Locked Widget
  (bind _returnvalue (`|CreateWidget` "/Game/BluePrints/Widget_BP/Doors/WBP_DoorIsLocked.WBP_DoorIsLocked_C"))
  (`UserWidget.AddToViewport` _returnvalue 0)
  (`GameplayStatics.PlaySoundAtLocation` (`self.LockedSound`) (`SceneComponent.K2_GetComponentLocation` (`self.Door`)) (struct) 1.0 1.0 0.0 null null null null))

(event `CheckForKey`
  ;[0.1046 0.03168 0.15 0.5] Checking for Key
  (for _array_element (`/Game/FirstPerson/Blueprints/BP_FirstPersonCharacter.Keys` (`self.Player Ref`))
    _)
  (if (`KismetTextLibrary.EqualEqual_TextText` _array_element (`self.DoorKeyID`))
    (`self.UnlockDoor`)
    (else
      (`self.DoorIsLocked`))))

(event `UnlockDoor`
  (bind _unlock_sound (`self.Unlock Sound`))
  ;[0.04622 0.0529 0.15 0.5] Unlock Door
  (set `self.Locked?` false)
  (`GameplayStatics.PlaySoundAtLocation` _unlock_sound (`SceneComponent.K2_GetComponentLocation` (`self.Door`)) (struct) 1.0 1.0 0.0 null null null null)
  (`KismetSystemLibrary.Delay` (`SoundBase.Duration` _unlock_sound))
  (`self.OpenCloseDoor`))

(event `OpenCloseDoor`
  ; Open Close Door
  (`self.Sounds`)
  (if (`self.DoorClosed?`)
    (set `self.DoorClosed?` false)
    (set `self.DotProdcut` (`KismetMathLibrary.Dot_VectorVector` (`KismetMathLibrary.Normal` (- (`self.K2_GetActorLocation` self) (`self.K2_GetActorLocation` (`self.Player Ref`)))) (`self.GetActorRightVector` self)))
    (bind (_direction _alpha) (`Timeline|Door_TL` :!label _label)
      (:`Update`
        (`SceneComponent.K2_SetRelativeRotation` (`self.Door`) (`KismetMathLibrary.MakeRotator` 0.0 0.0 (`KismetMathLibrary.Lerp` 0.0 (`KismetMathLibrary.SelectFloat` -90.0 90.0 (>= (`self.DotProdcut`) 0.0)) _alpha)) false false)))
    (else
      (set `self.DoorClosed?` true)
      (goto _label :!via `Reverse`))))

(event `AutoClose`
  ;[0.15 0.08879 0.1062 0.5] Auto Close the Door
  (`KismetSystemLibrary.K2_SetTimerDelegate` (delegate `DoorAutoClose`) 2.0 true))

(event `DoorAutoClose`
  ;[0.15 0.08879 0.1062 0.5] Auto Close the Door
  (if (`self.DoorClosed?`)
    _
    (elif (> (`KismetMathLibrary.Vector_Distance` (`self.K2_GetActorLocation` (`self.Player Ref`)) (`self.K2_GetActorLocation`)) (`self.CloseDistance`))
      (`self.OpenCloseDoor`))))

(fn `initialise`)

(fn `Sounds`
  (bind _returnvalue (`SceneComponent.K2_GetComponentLocation` (`self.Door`)))
  (if (`self.Locked?`)
    (`GameplayStatics.PlaySoundAtLocation` (`self.LockedSound`) _returnvalue (struct) 1.0 1.0 0.0 null null null null)
    (elif (`self.DoorClosed?`)
      (`GameplayStatics.PlaySoundAtLocation` (`self.OpenSound`) _returnvalue (struct) 1.0 1.0 0.0 null null null null)
      (else
        (`GameplayStatics.PlaySoundAtLocation` (`self.ClosedSound`) _returnvalue (struct) 1.0 1.0 0.0 null null null null)))))

(fn `UserConstructionScript`
  (`parent.UserConstructionScript`))