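; BP_Box_Child is an interactable box Blueprint that switches a point light on and off.
; Its Interact event checks the LightOn flag, sets the PointLight's hidden-in-game state to match the new state and flips the flag.
; Each toggle also prints a debug string, and the construction script only calls the parent's.
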(event `/Game/BluePrints/BPI_PlayerInteract.Interact`
  (bind _pointlight (`self.PointLight`))
  ; Turn Light On and Off
  (if (`self.LightOn?`)
    (`SceneComponent.SetHiddenInGame` _pointlight true false)
    (`KismetSystemLibrary.PrintString` "lightoff")
    (set `self.LightOn?` false)
    (else
      (`SceneComponent.SetHiddenInGame` _pointlight false false)
      (`KismetSystemLibrary.PrintString` "lighton")
      (set `self.LightOn?` true))))

(fn `UserConstructionScript`
  (`parent.UserConstructionScript`))