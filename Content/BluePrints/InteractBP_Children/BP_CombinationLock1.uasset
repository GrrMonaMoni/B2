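; Interactable three-dial combination padlock for an upstairs puzzle.
; It spawns BP_Dial1 actors on sockets; Interact toggles a lit close-up view that freezes the player, shows the cursor and routes clicks through a widget interaction component.
; Checkeveryturn compares dial numbers with LockCombo.
; A match plays a sound and lowers a lock component by timeline, then exits the view, destroys lock and dials, and signals puzzle completion.
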(event `self.ReceiveBeginPlay`
  ;[0.07084 0.06943 0.15 0.5] Spawn and Attach Dials + Spawn Light
  (`|ExecutionSequence`
    (:`then_0`
      (for _index (range 3)
        (bind _returnvalue (`|SpawnActorFromClass` "/Game/BluePrints/BP_Dial1.BP_Dial1_C" (`KismetMathLibrary.MakeTransform` (0.0 0.0 0.0)) "Undefined" "MultiplyWithRoot" null _index self null))
        (`KismetArrayLibrary.Array_Add` (`self.Dials`) _returnvalue)
        (`self.K2_AttachToComponent` _returnvalue (`self.re`) (select `int` _index :`0` "Dial01" :`1` "Dial02" :`2` "Dial03" :!type "Name") "KeepRelative" "KeepRelative" "KeepRelative" true)))
    (:`then_1`
      (`SceneComponent.SetVisibility` (`self.RectLight`) false false))))

(event `self.Interact`
  (bind _returnvalue (`GameplayStatics.GetPlayerController` 0))
  ;[0.15 0.06881 0.08467 0.5] Open/Close Padlock
  (`/Engine/EditorBlueprintResources/StandardMacros.FlipFlop`
    (:`A`
      (`PlayerController.SetViewTargetWithBlend` (`GameplayStatics.GetPlayerController` 0) self 1.0 "VTBlend_Linear" 0.0 false)
      (`SceneComponent.SetVisibility` (`self.RectLight`) true false)
      (`CharacterMovementComponent.DisableMovement` (`Character.CharacterMovement` (`GameplayStatics.GetPlayerCharacter` 0)))
      (`Controller.SetIgnoreLookInput` _returnvalue true)
      (`KismetSystemLibrary.Delay` 1.0)
      (`self.EnableInput` _returnvalue)
      (set `PlayerController.bShowMouseCursor` true _returnvalue)
      (bind _returnvalue_2 (`|CreateWidget` "/Game/BluePrints/Widget_BP/Lock/WBP_Doubleclicklock.WBP_Doubleclicklock_C"))
      (`UserWidget.AddToViewport` _returnvalue_2 0))
    (:`B`
      (`self.ExitView`)
      (`SceneComponent.SetVisibility` (`self.RectLight`) false false))))

(event `ExitView`
  (bind _returnvalue (`GameplayStatics.GetPlayerController` 0))
  (bind _returnvalue_2 (`GameplayStatics.GetPlayerCharacter` 0))
  ;[0.15 0.09412 0.03706 0.5] Reset View when Exiting
  (`PlayerController.SetViewTargetWithBlend` _returnvalue _returnvalue_2 1.0 "VTBlend_Linear" 0.0 false)
  (`self.DisableInput` _returnvalue)
  (`Controller.ResetIgnoreLookInput` _returnvalue)
  (set `PlayerController.bShowMouseCursor` false _returnvalue)
  (`CharacterMovementComponent.SetMovementMode` (`Character.CharacterMovement` _returnvalue_2) "MOVE_Walking" 0))

(event `Checkeveryturn`
  ;[0.07115 0.15 0.1035 0.5] Check Numbers
  (bind _localsuccess1 (`self.CheckCode`))
  (if _localsuccess1
    (`self.UnlockLock`)))

(event `Key|LeftMouseButton`
  (params (Key :type "Key Structure"))
  (bind _widgetinteraction (`self.WidgetInteraction`))
  ;[0.1279 0.15 0.05697 0.5] Make the dials clickable
  (:`Pressed`
    (`WidgetInteractionComponent.PressPointerKey` _widgetinteraction "LeftMouseButton"))
  (:`Released`
    (`WidgetInteractionComponent.ReleasePointerKey` _widgetinteraction "LeftMouseButton")))

(event `UnlockLock`
  ;[0.15 0.04677 0.1405 0.5] Unlock the Padlock
  (`GameplayStatics.PlaySound2D` "/Engine/EngineSounds/1kSineTonePing.1kSineTonePing" 1.0 1.0 0.0 null null)
  (bind (_direction _newtrack_0) (`Timeline|Unlock_TL` :!via `PlayFromStart`)
    (:`Update`
      (`SceneComponent.K2_SetRelativeLocation` (`self.re`) (`KismetMathLibrary.MakeVector` 0.0 0.0 (`KismetMathLibrary.Lerp` 0.0 -2.0 _newtrack_0)) false false)
      (`KismetSystemLibrary.Delay` 1.0)
      (`self.ExitView`)
      (`self.K2_DestroyActor` (`self.Dials`))
      (`self.K2_DestroyActor`)
      (`self.Upstairs Puzzle Completed`))))

(fn `CheckCode`
  (returns (LocalSuccess1 :type Boolean))
  (locals (Success :type Boolean))
  (for (_array_element _array_index) (`self.Dials`)
    (if (== (`/Game/BluePrints/BP_Dial1.Number` _array_element) (`|GetArrayItem` (`self.LockCombo`) _array_index))
      (set `local.Success` true)
      (else
        (set `local.Success` false)
        (break))))
  (return (`local.Success`)))

(fn `UserConstructionScript`
  (`parent.UserConstructionScript`))