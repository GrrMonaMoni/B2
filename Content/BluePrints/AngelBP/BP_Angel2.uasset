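; BP_Angel2 is a Weeping Angel-style enemy that chases the player while unseen and kills on contact.
; Each Tick, a dot product tests whether the angel lies within the player's forward cone, then a visibility trace runs from the camera to its head socket.
; It moves toward the player when outside the cone or the trace is blocked, and otherwise stops immediately.
; Its KillBox overlap calls Death on BP_FirstPersonCharacter, marked as testing.
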(event `self.ReceiveTick`
  (params (DeltaSeconds :type "Float (single-precision)"))
  (bind _returnvalue (`GameplayStatics.GetPlayerCharacter` 0))
  ; Looking at angel
  (if (> (`KismetMathLibrary.Dot_VectorVector` (`KismetMathLibrary.Normal` (- (`self.K2_GetActorLocation`) (`self.K2_GetActorLocation` _returnvalue))) (`self.GetActorForwardVector` _returnvalue)) 0.5)
    (bind (_outhits _returnvalue_2) (`KismetSystemLibrary.LineTraceMulti` (`PlayerCameraManager.GetCameraLocation` (`GameplayStatics.GetPlayerCameraManager` 0)) (`SceneComponent.GetSocketLocation` (`self.SkeletalMesh`) "head") "TraceTypeQuery1"))
    (if _returnvalue_2
      (`|AIMoveTo` self (0.0 0.0 0.0) (`GameplayStatics.GetPlayerCharacter` 0) :!label _label)
      (else
        (`MovementComponent.StopMovementImmediately` (`self.CharacterMovement`))))
    (else
      (goto _label))))

(event `self.Kill Box.OnComponentBeginOverlap`
  (params (OverlappedComponent :type "PrimitiveComponent Object Reference") (OtherActor :type "Actor Object Reference") (OtherComp :type "PrimitiveComponent Object Reference") (OtherBodyIndex :type Integer) (bFromSweep :type Boolean) (SweepResult :type "HitResult Structure (by ref)"))
  ; Kill (testing)
  (bind _asbp_first_person_character (cast `/Game/FirstPerson/Blueprints/BP_FirstPersonCharacter` OtherActor))
  (`/Game/FirstPerson/Blueprints/BP_FirstPersonCharacter.Death` _asbp_first_person_character))

(fn `UserConstructionScript`)