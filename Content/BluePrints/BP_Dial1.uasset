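; BP_Dial1 is a rotating number dial for a combination lock, with an arrow widget that receives a reference to it on BeginPlay.
; RotateDial plays a click sound and uses a timeline to yaw the mesh one tenth of a turn, ignoring input until it finishes.
; Each finished turn wraps at a full circle, derives Number from the angle and has the referenced lock run its check.
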(event `FindNumber`
  ;[0.15 0.03565 0.06904 0.5] Check current number
  (set `self.Number` (`KismetMathLibrary.FTrunc` (/ (`self.DialRotation`) 36.0))))

(event `RotateDial`
  ;[0.08428 0.15 0.05904 0.5] Rotate the dial
  (if (`self.CanRotate`)
    (set `self.CanRotate` false)
    (`GameplayStatics.PlaySound2D` "/Engine/VREditor/Sounds/UI/Flashlight_Switch.Flashlight_Switch" 1.0 1.0 0.0 null null)
    (bind (_direction _alpha) (`Timeline|DialRotation_TL` :!via `PlayFromStart`)
      (:`Update`
        (bind _returnvalue (+ (`self.DialRotation`) (`KismetMathLibrary.Lerp` 0.0 36.0 _alpha)))
        (`SceneComponent.K2_SetRelativeRotation` (`self.SM_DIalV3`) (`KismetMathLibrary.MakeRotator` 0.0 0.0 _returnvalue) false false))
      (:`Finished`
        (set `self.DialRotation` _returnvalue)
        (if (>= (`self.DialRotation`) 360.0)
          (set `self.DialRotation` 0.0)
          (`SceneComponent.K2_SetRelativeRotation` :`self` (`self.SM_DIalV3`)))
        (`self.FindNumber`)
        (`/Game/BluePrints/InteractBP_Children/BP_CombinationLock1.Checkeveryturn` (`self.LockRef`))
        (set `self.CanRotate` true)))))

(event `self.ReceiveBeginPlay`
  ;[0.15 0.1112 0.05237 0.5] Show Dial Arrows
  (bind _aswbp_lock_arrow_1 (cast `/Game/BluePrints/Widget_BP/Lock/WBP_LockArrow1` (`WidgetComponent.GetUserWidgetObject` (`self.Widget`))))
  (`/Game/BluePrints/Widget_BP/Lock/WBP_LockArrow1.Initalise2` _aswbp_lock_arrow_1 self))

(fn `UserConstructionScript`)