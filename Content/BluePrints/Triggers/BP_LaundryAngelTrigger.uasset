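; BP_LaundryAngelTrigger is a one-shot scare that swaps a posed angel mesh for a live AI angel.
; Leaving Trigger1 runs a timeline that turns the skeletal mesh to a fixed facing with a laugh sound.
; Entering Trigger plays a sound, briefly delays, hides the mesh and spawns BP_Angel2 at hardcoded coordinates.
; DoOnce gates both overlaps, which do not filter the overlapping actor; a second timeline branch is never run.
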(event `self.Trigger.OnComponentBeginOverlap`
  (params (OverlappedComponent :type "PrimitiveComponent Object Reference") (OtherActor :type "Actor Object Reference") (OtherComp :type "PrimitiveComponent Object Reference") (OtherBodyIndex :type Integer) (bFromSweep :type Boolean) (SweepResult :type "HitResult Structure (by ref)"))
  (bind _skeletalmesh (`self.SkeletalMesh`))
  ; Turn to face the player
  (`/Engine/EditorBlueprintResources/StandardMacros.DoOnce` false
    (:`Completed`
      (`GameplayStatics.PlaySoundAtLocation` "/Game/Sounds/Door/Locked.Locked" (`SceneComponent.K2_GetComponentLocation` _skeletalmesh) (struct) 1.5 1.0 0.0 null null null null)
      (`KismetSystemLibrary.Delay` 0.2)
      (`SceneComponent.SetVisibility` _skeletalmesh false false)
      (`AIBlueprintHelperLibrary.SpawnAIFromClass` "/Game/BluePrints/AngelBP(WORKING)/BP_Angel2.BP_Angel2_C" null (1182.154582 -7902.070894 88.00012) (struct :`Yaw` 68.0) false null))))

(event `self.Trigger1.OnComponentEndOverlap`
  (params (OverlappedComponent :type "PrimitiveComponent Object Reference") (OtherActor :type "Actor Object Reference") (OtherComp :type "PrimitiveComponent Object Reference") (OtherBodyIndex :type Integer))
  (bind _skeletalmesh (`self.SkeletalMesh`))
  ; Face the Player
  (`/Engine/EditorBlueprintResources/StandardMacros.DoOnce` false
    (:`Completed`
      (bind (_direction _turn) (`Timeline|Timeline` :!via `PlayFromStart`)
        (:`Update`
          (bind _output_get (set `self.Ref1` (`self.K2_GetActorRotation`)))
          (`SceneComponent.K2_SetWorldRotation` _skeletalmesh (`KismetMathLibrary.RLerp` _output_get (struct :`Yaw` -115.0) _turn) false false)
          (`/Engine/EditorBlueprintResources/StandardMacros.DoOnce` false
            (:`Completed`
              (`GameplayStatics.PlaySoundAtLocation` "/Game/Sounds/FoleyEffects/Laughing/Laughing_7EDITED.Laughing_7EDITED" (`SceneComponent.K2_GetComponentLocation` _skeletalmesh) (struct) 1.0 1.0 0.0 null null null null))))))))

(fn `UserConstructionScript`)