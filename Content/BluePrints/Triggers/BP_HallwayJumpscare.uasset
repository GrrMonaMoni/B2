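; BP_HallwayJumpscare is a one-shot jumpscare, an AI-moved pawn triggered when the player character overlaps its box.
; It plays a laughing sound at its mesh's location and starts an AI move toward the BP_PointB actor in the level.
; The destroy timer runs from the start of the move rather than its completion, so the pawn vanishes one second later whether or not it arrives.
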(event `self.Box.OnComponentBeginOverlap`
  (params (OverlappedComponent :type "PrimitiveComponent Object Reference") (OtherActor :type "Actor Object Reference") (OtherComp :type "PrimitiveComponent Object Reference") (OtherBodyIndex :type Integer) (bFromSweep :type Boolean) (SweepResult :type "HitResult Structure (by ref)"))
  ;[0.05843 0.15 0.03376 0.5] Play Sound + Move Angel
  (if (== OtherActor (`GameplayStatics.GetPlayerCharacter` 0))
    (`/Engine/EditorBlueprintResources/StandardMacros.DoOnce` false
      (:`Completed`
        (`GameplayStatics.SpawnSoundAtLocation` "/Game/Sounds/FoleyEffects/Laughing/Laughing_2EDITED.Laughing_2EDITED" (`SceneComponent.K2_GetComponentLocation` (`self.Mesh`)) (struct) 0.7 0.9 0.0 null null)
        (bind _returnvalue (`GameplayStatics.GetActorOfClass` "/Game/BluePrints/Triggers/BP_PointB.BP_PointB_C"))
        (`|AIMoveTo` self (`self.K2_GetActorLocation` _returnvalue) null
          (:`then`
            (`KismetSystemLibrary.Delay` 1.0)
            (`self.K2_DestroyActor`)))))))

(fn `UserConstructionScript`)